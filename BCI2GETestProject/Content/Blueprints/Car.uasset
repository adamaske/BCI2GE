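; Simple car actor that slides along its local axes at its current Velocity, applied every Tick as an unswept offset scaled by delta time.
; TurnLeft and TurnRight replace Velocity with pure sideways motion scaled by Strength, using a hard-coded rate for left and the Speed variable for right.
; Both print a duplicated "turning left" debug message, and SetVelocity assigns any vector directly.
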(event EventBeginPlay)

(event Collision|EventActorBeginOverlap
  (params (OtherActor :type Actor%20Object%20Reference)))

(event EventTick
  (params (DeltaSeconds :type Float%20%28single-precision%29))
  (Transformation|AddActorLocalOffset self (* (Variables|Default|GetVelocity) DeltaSeconds) false false))

(fn ConstructionScript)

(fn TurnLeft
  (params (strength :type Float%20%28double-precision%29))
  (bind _returnvalue (Utilities|String|ToString(Float) strength))
  (bind _returnvalue_2 (Utilities|String|Append "Car is turning left, with multiplier: " _returnvalue))
  (Variables|Default|SetVelocity (Math|Vector|MakeVector 0.0 (* strength -1e+02) 0.0))
  (Development|PrintString _returnvalue_2)
  (Development|PrintString _returnvalue_2))

(fn TurnRight
  (params (strength :type Float%20%28double-precision%29))
  (bind _returnvalue (Utilities|String|ToString(Float) strength))
  (bind _returnvalue_2 (Utilities|String|Append "Car is turning left, with multiplier: " _returnvalue))
  (Variables|Default|SetVelocity (Math|Vector|MakeVector 0.0 (* strength (Variables|Default|GetSpeed)) 0.0))
  (Development|PrintString _returnvalue_2)
  (Development|PrintString _returnvalue_2))

(fn SetVelocity
  (params (vec :type Vector))
  (Variables|Default|SetVelocity vec))