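; BPCarGameSceneController is a scene controller that sets up the view for a car game when play begins.
; On BeginPlay it checks for valid Car and Camera references, aims the camera at the car through LookAtStill, makes it the player's view target and sets IsPlaying.
; A missing reference prints a message and clears IsPlaying; Tick checks the flag but does nothing yet.
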(event EventBeginPlay
  (bind _camera (Variables|Default|GetCamera))
  (if (Utilities|IsValid (Variables|Default|GetCar))
    (if (Utilities|IsValid (Variables|Default|GetCamera))
      (Variables|Default|SetIsPlaying true)
      (Default|LookatStill _camera (Utilities|ResolveSoftReference (Variables|Default|GetCar)) "0, 0, 0")
      (Game|Player|SetViewTargetwithBlend (Game|GetPlayerController 0) _camera 0.0 "VTBlend_Linear" 0.0 false)
      (else
        (Development|PrintString "No Camera, no play")
        (Variables|Default|SetIsPlaying false)))
    (else
      (Development|PrintString "No Car, no play")
      (Variables|Default|SetIsPlaying false))))

(event Collision|EventActorBeginOverlap
  (params (OtherActor :type Actor%20Object%20Reference)))

(event EventTick
  (params (DeltaSeconds :type Float%20%28single-precision%29))
  (if (Variables|Default|GetIsPlaying)
    _))

(fn ConstructionScript)